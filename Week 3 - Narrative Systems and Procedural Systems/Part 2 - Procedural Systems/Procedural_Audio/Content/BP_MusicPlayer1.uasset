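; BP_MusicPlayer1 is an interactive music actor that changes its audio in response to overlaps with three trigger volumes.
; The BPM and Crossfade triggers set matching float parameters on the Audio component when entered and reset them on exit.
; Entering the Melody trigger sends a NewMelody trigger parameter, leaving the musical response to the sound asset driven by these parameters.
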(event OnComponentBeginOverlap(Trigger_BPM)
  (params (OverlappedComponent :type Primitive%20Component%20Object%20Reference) (OtherActor :type Actor%20Object%20Reference) (OtherComp :type Primitive%20Component%20Object%20Reference) (OtherBodyIndex :type Integer) (bFromSweep :type Boolean) (SweepResult :type Hit%20Result%20Structure%20%28by%20ref%29))
  (Audio|Parameter|SetFloatParameter (Variables|Default|GetAudio) "BPM" 1.2e+02 :!class /Script/Engine.AudioComponent))

(event OnComponentEndOverlap(Trigger_BPM)
  (params (OverlappedComponent :type Primitive%20Component%20Object%20Reference) (OtherActor :type Actor%20Object%20Reference) (OtherComp :type Primitive%20Component%20Object%20Reference) (OtherBodyIndex :type Integer))
  (Audio|Parameter|SetFloatParameter (Variables|Default|GetAudio) "BPM" 9e+01 :!class /Script/Engine.AudioComponent))

(event OnComponentBeginOverlap(Trigger_Crossfade)
  (params (OverlappedComponent :type Primitive%20Component%20Object%20Reference) (OtherActor :type Actor%20Object%20Reference) (OtherComp :type Primitive%20Component%20Object%20Reference) (OtherBodyIndex :type Integer) (bFromSweep :type Boolean) (SweepResult :type Hit%20Result%20Structure%20%28by%20ref%29))
  (Audio|Parameter|SetFloatParameter (Variables|Default|GetAudio) "Crossfade" 1.0 :!class /Script/Engine.AudioComponent))

(event OnComponentEndOverlap(Trigger_Crossfade)
  (params (OverlappedComponent :type Primitive%20Component%20Object%20Reference) (OtherActor :type Actor%20Object%20Reference) (OtherComp :type Primitive%20Component%20Object%20Reference) (OtherBodyIndex :type Integer))
  (Audio|Parameter|SetFloatParameter (Variables|Default|GetAudio) "Crossfade" 0.0 :!class /Script/Engine.AudioComponent))

(event OnComponentBeginOverlap(Trigger_Melody)
  (params (OverlappedComponent :type Primitive%20Component%20Object%20Reference) (OtherActor :type Actor%20Object%20Reference) (OtherComp :type Primitive%20Component%20Object%20Reference) (OtherBodyIndex :type Integer) (bFromSweep :type Boolean) (SweepResult :type Hit%20Result%20Structure%20%28by%20ref%29))
  (Class|AudioParameterControllerInterface|SetTriggerParameter(Message) (Variables|Default|GetAudio) "NewMelody"))

(event EventBeginPlay)

(event Collision|EventActorBeginOverlap
  (params (OtherActor :type Actor%20Object%20Reference)))

(event EventTick
  (params (DeltaSeconds :type Float%20%28single-precision%29)))

(fn ConstructionScript)